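; BP_MCPlayerController is a player controller that toggles the inventory screen with the E key.
; A FlipFlop on the key press alternates between showing and hiding the inventory through the MCHUD.
; Opening switches input to Game and UI and shows the mouse cursor, while closing restores game-only input and hides it.
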(event `Key|E`
  (params (Key :type "Key Structure"))
  (bind _returnvalue (`self.GetHUD`))
  (:`Pressed`
    (`/Engine/EditorBlueprintResources/StandardMacros.FlipFlop`
      (:`A`
        (bind _asmchud (cast `MCHUD` _returnvalue))
        (`MCHUD.ShowInventory` _asmchud)
        (`WidgetBlueprintLibrary.SetInputMode_GameAndUIEx` self null)
        (set `self.bShowMouseCursor` true))
      (:`B`
        (bind _asmchud_2 (cast `MCHUD` _returnvalue))
        (`MCHUD.HideInventory` _asmchud_2)
        (`WidgetBlueprintLibrary.SetInputMode_GameOnly` self)
        (set `self.bShowMouseCursor` false)))))

(fn `UserConstructionScript`)