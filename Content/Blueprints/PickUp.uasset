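; Dropped item pickup for a block world that shows a small randomly scattered stack of instanced meshes, spinning and bobbing.
; When Falling is called, its box simulates physics until a short downward trace hits a Chunk, then physics stops and the sphere's pawn-detecting collision is set.
; A FirstPersonCharacter overlap makes it interpolate toward the player each Tick, hand over ItemBaseData via PickItem, and destroy itself.
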(event `self.ReceiveBeginPlay`)

(event `self.ReceiveTick`
  (params (DeltaSeconds :type "Float (single-precision)"))
  (bind _returnvalue (`self.K2_GetActorLocation`))
  (bind _returnvalue_2 (`self.K2_GetActorLocation` (`self.First Person Character`)))
  ;[1 1 1] 旋转浮动
  (`|ExecutionSequence`
    (:`then_0`
      (`self.FloatAndRotate`))
    (:`then_1`
      (`self.CheckIsFalling`))
    (:`then_2`
      (if (`self.IsPickingUp`)
        (`self.K2_SetActorLocation` (`KismetMathLibrary.VInterpTo` _returnvalue _returnvalue_2 1.0 0.3))
        (if (== _returnvalue _returnvalue_2 :`ErrorTolerance` 10.0)
          (`/Game/Blueprints/FirstPersonCharacter.Pick Item` (`self.First Person Character`) (`self.ItemBaseData`))
          (`self.K2_DestroyActor`))))))

(event `self.Sphere.OnComponentBeginOverlap`
  (params (OverlappedComponent :type "PrimitiveComponent Object Reference") (OtherActor :type "Actor Object Reference") (OtherComp :type "PrimitiveComponent Object Reference") (OtherBodyIndex :type Integer) (bFromSweep :type Boolean) (SweepResult :type "HitResult Structure (by ref)"))
  (bind _asfirst_person_character (cast `/Game/Blueprints/FirstPersonCharacter` OtherActor))
  (set `self.First Person Character` _asfirst_person_character)
  (set `self.IsPickingUp` true))

(fn `CheckIsFalling`
  (if (`self.IsFalling`)
    (bind _onfloor (`self.IsOnFloor`))
    (if _onfloor
      (`PrimitiveComponent.SetSimulatePhysics` (`self.Box`) false)
      (`PrimitiveComponent.SetCollisionProfileName` (`self.Sphere`) "OnlyCarePawn" true) ; 初始时关闭此碰撞，落地后开启人物检测的碰撞
      (set `self.IsFalling` false))))

(fn `Falling`
  (set `self.IsFalling` true)
  (`PrimitiveComponent.SetSimulatePhysics` (`self.Box`) true))

(fn `FloatAndRotate`
  (bind _instancedstaticmesh (`self.InstancedStaticMesh`))
  (`SceneComponent.K2_AddRelativeRotation` _instancedstaticmesh (struct :`Yaw` 1.0) false false)
  (`SceneComponent.K2_SetRelativeLocation` _instancedstaticmesh (`KismetMathLibrary.MakeVector` 0.0 0.0 (* (`KismetMathLibrary.Sin` (* (`self.GetGameTimeSinceCreation`) (`self.FloatSpeed`))) (`self.FloatAmplitude`))) false false))

(fn `IsOnFloor`
  (returns (OnFloor :type Boolean))
  (bind _returnvalue (`self.K2_GetActorLocation`))
  (bind _outhit (`KismetSystemLibrary.LineTraceSingle` :`Start` _returnvalue :`End` (- _returnvalue (0.0 0.0 20.0)) :`TraceChannel` "TraceTypeQuery1" :`DrawTime` 1.0))
  (cast `Chunk` (`.HitActor` (`GameplayStatics.BreakHitResult` _outhit))
    (:`then`
      (return true))
    (:`CastFailed`
      (return false))))

(fn `UserConstructionScript`
  (bind _instancedstaticmesh (`self.InstancedStaticMesh`))
  (bind (_assetdata_icon _assetdata_mesh _assetdata_material) (break `ItemAssetData` (`self.AssetData`)))
  (bind (_itembasedata_itemtype _itembasedata_amount) (break `ItemBase` (`self.ItemBaseData`)))
  (`StaticMeshComponent.SetStaticMesh` _instancedstaticmesh _assetdata_mesh)
  (`PrimitiveComponent.SetMaterial` _instancedstaticmesh 0 _assetdata_material)
  (for _ (range (+ (`KismetMathLibrary.Min` (- _itembasedata_amount 1) 3) 1))
    (`InstancedStaticMeshComponent.AddInstance` (`self.InstancedStaticMesh`) (`KismetMathLibrary.MakeTransform` (`KismetMathLibrary.MakeVector` (`KismetMathLibrary.RandomFloatInRange` -10.0 10.0) (`KismetMathLibrary.RandomFloatInRange` -10.0 10.0) (`KismetMathLibrary.RandomFloatInRange` 0.0 20.0))))))